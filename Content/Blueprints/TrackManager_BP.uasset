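; TrackManager_BP is a race manager that tracks the AI and player machines and starts the race for them.
; UpdateMachines fills separate arrays with every AdaptativeMachine and PlayerMachine actor found in the world.
; StartRace loops over both cached arrays and sends each machine StartRaceMessage.
; BeginPlay and Tick are empty, so both operations depend on their events being called.
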(event Custom|UpdateMachines
  (bind _outactors (Actor|GetAllActorsOfClass "/Script/ZeroProject.AdaptativeMachine"))
  (Variables|Default|SetAIMachines _outactors)
  (bind _outactors_2 (Actor|GetAllActorsOfClass "/Script/ZeroProject.PlayerMachine"))
  (Variables|Default|SetPlayersMachines _outactors_2))

(event EventBeginPlay)

(event EventTick
  (params (DeltaSeconds :type Float%20%28single-precision%29)))

(event EventStartRace
  (for _array_element (Variables|Default|GetAIMachines)
    (Class|Machine|StartRace(Message) _array_element))
  (for _array_element_2 (Variables|Default|GetPlayersMachines)
    (Class|Machine|StartRace(Message) _array_element_2)))