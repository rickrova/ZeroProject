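; FinalLapVerification_BP is a trigger actor that lets a referenced Goal validate a lap once the player has passed through it.
; When player pawn 0 begins overlapping it, it sets the Goal's CanCheckLap flag to true.
; Enable and Disable events switch the actor on and off by setting its scale to one or zero rather than toggling collision.
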(event Custom|Disable
  (Transformation|SetActorScale3D "0, 0, 0"))

(event Custom|Enable
  (Transformation|SetActorScale3D "1.000000,1.000000,1.000000"))

(event EventBeginPlay
  (|CallParentFunction) ; This node is disabled and will not be called.\nDrag off pins to build functionality.
)

(event Collision|EventActorBeginOverlap
  (params (OtherActor :type Actor%20Object%20Reference))
  (if (== OtherActor (Game|Player|GetPlayerPawn 0))
    (Variables|/Game/Blueprints/Test/Goal_BP.Goal_BP_C|SetCanCheckLap (Variables|Default|GetGoal) true)))

(event EventTick
  (params (DeltaSeconds :type Float%20%28single-precision%29)))

(fn ConstructionScript
  (|CallParentFunction))