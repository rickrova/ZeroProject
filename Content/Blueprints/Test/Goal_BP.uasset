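; Goal_BP is a test goal actor that detects when the player crosses it, apparently as a lap line.
; On overlap with player 0's pawn, it calls Disable on FinalLapVerification, then prints "Lap" if CanCheckLap is true.
; It only reads CanCheckLap and keeps no lap count; BeginPlay, Tick and the construction script add no logic.
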(event EventBeginPlay
  (|CallParentFunction) ; This node is disabled and will not be called.\nDrag off pins to build functionality.
)

(event Collision|EventActorBeginOverlap
  (params (OtherActor :type Actor%20Object%20Reference))
  (|CallParentFunction 0)
  (if (== OtherActor (Game|Player|GetPlayerPawn 0))
    (Default|Disable (Variables|Default|GetFinalLapVerification))
    (if (Variables|Default|GetCanCheckLap)
      (Development|PrintString "Lap"))))

(event EventTick
  (params (DeltaSeconds :type Float%20%28single-precision%29))
  (|CallParentFunction DeltaSeconds) ; This node is disabled and will not be called.\nDrag off pins to build functionality.
)

(fn ConstructionScript
  (|CallParentFunction))