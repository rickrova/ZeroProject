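; Race position controller that ranks the AI machines and the player every tick and sends the player's place to the main UI.
; AI machines report their covered distance, while the player's is estimated from the closest spline input key plus completed laps.
; A jump in the player's distance beyond a threshold counts as a new lap.
; Ranking repeatedly extracts the maximum distance, then finds the player by the display name "Machine".
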(event Custom|Init
  (params (AIMachines :type Array%20of%20AI%20Machine%20Blueprint%20Object%20References) (PlayerMachine :type Kinematic%20Machine%20Object%20Reference) (Spline :type Spline%20Actor%20Object%20Reference) (MainUI :type Main%20UI%20BP%20Object%20Reference))
  (bind _output_get (Variables|Default|SetMainUI MainUI))
  (bind _output_get_2 (Variables|/Game/Blueprints/UI/MainUI_BP.MainUI_BP_C|SetAIMachines _output_get AIMachines))
  (Variables|Default|SetSplineActor Spline)
  (Variables|Default|SetPlayerMachine PlayerMachine)
  (bind _output_get_3 (Variables|Default|SetRacers _output_get_2))
  (Utilities|Array|Add _output_get_3 (Variables|Default|GetPlayerMachine))
  (Variables|/Game/Blueprints/UI/MainUI_BP.MainUI_BP_C|SetPlayerMachine (Variables|Default|GetMainUI) (Variables|Default|GetPlayerMachine)))

(event EventBeginPlay)

(event EventTick
  (params (DeltaSeconds :type Float%20%28single-precision%29))
  (bind _laplength (Variables|Default|GetLapLength))
  (bind _rawvalues (Variables|Default|GetRawValues))
  (bind (_indexofmaxvalue _maxvalue) (Math|Float|MaxOfFloatArray _rawvalues))
  (Utilities|Array|Clear (Variables|Default|GetSorted))
  (Utilities|Array|Clear (Variables|Default|GetRawValues))
  (Utilities|Array|Clear (Variables|Default|GetSortedValues))
  (for _array_element (Variables|Default|GetRacers)
    (bind _asaimachine_blueprint (Utilities|Casting|CastToAIMachine_Blueprint _array_element)
      (:then
        (Utilities|Array|Add (Variables|Default|GetRawValues) (Variables|/Script/ZeroProject.AIMachine|GetCoveredDistance _asaimachine_blueprint)))
      (:CastFailed
        (bind _askinematic_machine (Utilities|Casting|CastToKinematicMachine _array_element))
        (Utilities|Array|Add (Variables|Default|GetRawValues) (+ (* (Class|SplineComponent|FindInputKeyClosesttoWorldLocation (Variables|/Script/ZeroProject.SplineActor|GetSpline (Variables|Default|GetSplineActor)) (Transformation|GetWorldLocation (Variables|/Script/ZeroProject.KinematicMachine|GetKinematicComponent _askinematic_machine))) 10.02) (* _laplength (Variables|Default|GetLapCount))))
        (bind _output_get (Variables|Default|SetDeltaLocation (- (+ (* (Class|SplineComponent|FindInputKeyClosesttoWorldLocation (Variables|/Script/ZeroProject.SplineActor|GetSpline (Variables|Default|GetSplineActor)) (Transformation|GetWorldLocation (Variables|/Script/ZeroProject.KinematicMachine|GetKinematicComponent _askinematic_machine))) 10.02) (* _laplength (Variables|Default|GetLapCount))) (Variables|Default|GetLastLocation))))
        (Variables|Default|SetLastLocation (+ (* (Class|SplineComponent|FindInputKeyClosesttoWorldLocation (Variables|/Script/ZeroProject.SplineActor|GetSpline (Variables|Default|GetSplineActor)) (Transformation|GetWorldLocation (Variables|/Script/ZeroProject.KinematicMachine|GetKinematicComponent _askinematic_machine))) 10.02) (* _laplength (Variables|Default|GetLapCount))))
        (if (> (Math|Float|Absolute(Float) _output_get) (Variables|Default|GetDeltaThereshold))
          (Variables|Default|SetLapCount (+ (Variables|Default|GetLapCount) 1))
          (Variables|Default|SetLastLocation (+ (Variables|Default|GetLastLocation) _laplength))))))
  (for _index (range 0 (Utilities|Array|LastIndex (Variables|Default|GetRacers)))
    (Utilities|Array|Add (Variables|Default|GetSorted) (Utilities|GetDisplayName (Utilities|Array|Get(acopy) (Variables|Default|GetRacers) _indexofmaxvalue)))
    (Utilities|Array|Add (Variables|Default|GetSortedValues) _maxvalue)
    (Utilities|Array|SetArrayElem (Variables|Default|GetRawValues) _indexofmaxvalue -1.0))
  (for (_array_element_2 _array_index) (Variables|Default|GetSorted)
    (if (== _array_element_2 "Machine")
      (Default|SetSortedNames (Variables|Default|GetMainUI) (+ _array_index 1))))
  (if true
    _))