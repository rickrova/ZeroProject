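; Tricka is a Blueprint that sets up and starts races between AI-driven and player machines.
; SetupMachines gathers all AdaptativeMachine, PlayerMachine and SplineActor_BP actors in the world into stored arrays.
; StartRace sends StartRaceMessage to each stored AI machine, then to each player machine.
; The splines are only stored here, and neither custom event is called within this Blueprint.
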(event Custom|SetupMachines
  (bind _outactors (Actor|GetAllActorsOfClass "/Script/ZeroProject.AdaptativeMachine"))
  (Variables|Default|SetAIMachines _outactors)
  (bind _outactors_2 (Actor|GetAllActorsOfClass "/Script/ZeroProject.PlayerMachine"))
  (Variables|Default|SetPlayersMachines _outactors_2)
  (bind _outactors_3 (Actor|GetAllActorsOfClass "/Game/Blueprints/Test/SplineActor_BP.SplineActor_BP_C"))
  (Variables|Default|SetSplines _outactors_3))

(event EventBeginPlay)

(event Collision|EventActorBeginOverlap
  (params (OtherActor :type Actor%20Object%20Reference)))

(event EventTick
  (params (DeltaSeconds :type Float%20%28single-precision%29)))

(event EventStartRace
  (for _array_element (Variables|Default|GetAIMachines)
    (Class|Machine|StartRace(Message) _array_element))
  (for _array_element_2 (Variables|Default|GetPlayersMachines)
    (Class|Machine|StartRace(Message) _array_element_2)))

(fn ConstructionScript)